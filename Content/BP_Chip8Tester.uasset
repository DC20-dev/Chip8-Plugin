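; BP_Chip8Tester is a test Blueprint for driving a CHIP-8 emulator.
; It switches the Emulator on at BeginPlay.
; Events for hex keys 0 and 9 and for QUIT route through a shared Call event into the emulator's hex keyboard handler.
; Call always reports the key as released, so no key-down is ever sent.
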(event Custom|Call
  (params (key :type EEmulatorKeys%20Enum :default "K_0"))
  (Class|Chip8|HexKeyboardKeyEvent (Variables|Default|GetEmulator) key false))

(event Custom|9
  (CallFunction|Call "K_9"))

(event Custom|0
  (CallFunction|Call "K_0"))

(event Custom|QUIT
  (CallFunction|Call "K_QUIT"))

(event EventBeginPlay
  (Class|Chip8|SwitchON (Variables|Default|GetEmulator)))

(fn ConstructionScript)